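; Character system component that manages item slots in the player's inventory and a container inventory.
; AddToInventory caps items of two weapon types at two in total, printing a message and returning false, but certain swap types bypass the check.
; Slot helpers overwrite array entries by index with copied item data and zero quantity, while removal writes an empty slot.
; Container writes only happen for swaps from the player's inventory; CreateSlot is empty.
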(fn CreateSlot)

(fn AddtoSlot
  (params (Item :type Slot%20Structure%20Structure) (Index :type Integer))
  (bind _itemstruct (Utilities|Struct|BreakSlotStructure Item))
  (bind (_name _description _mesh _icon _itemtype) (Utilities|Struct|BreakItemStruct _itemstruct))
  (Utilities|Array|SetArrayElem (Variables|Default|GetInventory) Index (Utilities|Struct|MakeSlotStructure (Utilities|Struct|MakeItemStruct _name _description _mesh _icon _itemtype))))

(fn AddtoInventory
  (params (Item :type Slot%20Structure%20Structure) (Index :type Integer) (ItemSwappedType :type ItemType%20Enum :default "NewEnumerator0"))
  (bind _itemstruct (Utilities|Struct|BreakSlotStructure Item))
  (bind _itemtype (Utilities|Struct|BreakItemStruct _itemstruct))
  (if (or (Utilities|Enum|Equal(Enum) ItemSwappedType "NewEnumerator1") (Utilities|Enum|Equal(Enum) ItemSwappedType "NewEnumerator2"))
    (CallFunction|AddtoSlot Item Index)
    (return true)
    (elif (or (Utilities|Enum|Equal(Enum) _itemtype "NewEnumerator1") (Utilities|Enum|Equal(Enum) _itemtype "NewEnumerator2"))
      (Variables|Default|SetNbWeaponInInventory 0)
      (for _array_element (Variables|Default|GetInventory)
        (if (or (Utilities|Enum|Equal(Enum) (.ItemType (Utilities|Struct|BreakItemStruct (.ItemStruct (Utilities|Struct|BreakSlotStructure _array_element)))) "NewEnumerator1") (Utilities|Enum|Equal(Enum) (.ItemType (Utilities|Struct|BreakItemStruct (.ItemStruct (Utilities|Struct|BreakSlotStructure _array_element)))) "NewEnumerator2"))
          (Variables|Default|SetNbWeaponInInventory (+ (Variables|Default|GetNbWeaponInInventory) 1))))
      (if (>= (Variables|Default|GetNbWeaponInInventory) 2)
        (Development|PrintString "You already got 2 weapons in inventory" true true "(R=1.000000,G=0.833000,B=0.000000,A=1.000000)" 1e+01)
        (return false)
        (else
          (CallFunction|AddtoSlot Item Index)
          (return true)))
      (else
        (CallFunction|AddtoSlot Item Index)
        (return true)))))

(fn RemovefromInventory
  (params (Index :type Integer))
  (Utilities|Array|SetArrayElem :TargetArray (Variables|Default|GetInventory) :Index Index))

(fn AddtoContainerInventory
  (params (Item :type Slot%20Structure%20Structure) (Index :type Integer) (IsSwappedFromPlayerInventory? :type Boolean))
  (if IsSwappedFromPlayerInventory?
    (CallFunction|AddtoContainerSlot Item Index)))

(fn AddtoContainerSlot
  (params (Item :type Slot%20Structure%20Structure) (Index :type Integer))
  (bind _itemstruct (Utilities|Struct|BreakSlotStructure Item))
  (bind (_name _description _mesh _icon _itemtype) (Utilities|Struct|BreakItemStruct _itemstruct))
  (Utilities|Array|SetArrayElem (Variables|Default|GetContainerInventory) Index (Utilities|Struct|MakeSlotStructure (Utilities|Struct|MakeItemStruct _name _description _mesh _icon _itemtype))))