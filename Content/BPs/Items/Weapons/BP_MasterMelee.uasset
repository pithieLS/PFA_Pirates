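; Base melee weapon for player and AI characters, running a three-hit combo of random montages chosen by camera mode, with aim input setting parry.
; Gate and delays pace and reset the combo, while macros switch the player's movement between attack and walk rotation.
; In TPS, a looping timer turns the attacker toward a nearby enemy.
; HitDetect damages non-parrying characters overlapping a capsule, spawning impact effects, projectile and sound.
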(event Custom|PlayAttack
  (Utilities|FlowControl|Sequence
    (:then_0
      (Utilities|FlowControl|Gate false :!label _label
        (:Exit
          (Utilities|IsValid (Variables|Default|GetAs%20BP%20Player)
            (:Is%20Valid
              (Utilities|AttackMode
                (:Out
                  _)))
            (:Is%20Not%20Valid
              _))
          (if (Variables|Default|GetCanAttack)
            (Variables|Default|SetIsAttacking true)
            (Animation|Montage|PlayMontage (Utilities|SelectSM) (Utilities|GetAttack)
              (:then
                (bind _closestactor (CallFunction|GetClosestEnemy))
                (CallFunction|RotateTowardEnemy _closestactor)
                (bind _result (Math|Integer|IncrementInt (Variables|Default|GetAttackIndex))
                  (:%20%20
                    (bind _output_get (Variables|Default|SetAttackIndex _result))
                    (if (< _output_get 3)
                      (Variables|Default|SetCanAttack false)
                      (Utilities|FlowControl|Delay (Variables|Stats|GetAttackDelay))
                      (Variables|Default|SetCanAttack true)
                      (else
                        (Variables|Default|SetCanAttack false)
                        (Variables|Default|SetAttackIndex 0)
                        (Utilities|FlowControl|Sequence
                          (:then_0
                            (Utilities|FlowControl|Delay (Variables|Stats|GetStillAttackingDelay))
                            (Variables|Default|SetIsAttacking false)
                            (CallFunction|CanBeginAttack)
                            (Utilities|WalkMode))
                          (:then_1
                            (goto _label Close)))))))))))))
    (:then_1
      (Utilities|FlowControl|RetriggerableDelay (Variables|Stats|GetStillAttackingDelay))
      (Variables|Default|SetAttackIndex 0)
      (Variables|Default|SetIsAttacking false)
      (Utilities|WalkMode))))

(event Custom|CanBeginAttack
  (Variables|Default|SetCanAttack true)
  (Utilities|FlowControl|Gate false) ; enters at Open
)

(event Custom|HitDetect
  (bind _hitlocation (Variables|Default|GetHitLocation))
  (bind _as_bp_master_character (Variables|Default|GetAs%20BP%20Master%20Character))
  (bind _returnvalue (Transformation|GetWorldLocation _hitlocation))
  (bind _array_element (Utilities|Array|ForEachLoopwithBreak (Collision|GetOverlappingActors (Variables|Default|GetHitDetectionCapsule) "/Game/BPs/CharacterRelated/BP_MasterCharacter.BP_MasterCharacter_C" :!class /Script/Engine.PrimitiveComponent))
    (:LoopBody
      (if (and (Utilities|DoesObjectImplementInterface _array_element "/Game/BPs/Interfaces/BPI_Combat.BPI_Combat_C") (!= _array_element (Variables|Default|GetAs%20BP%20Master%20Character)))
        (if (not (Variables|/Game/BPs/CharacterRelated/BP_MasterCharacter.BP_MasterCharacter_C|GetIsParrying (.AsBP%20Master%20Character (Utilities|Casting|CastToBP_MasterCharacter _array_element))))
          (Class|BPICombat|DealDamages(Message) _as_bp_master_character _array_element (Variables|Stats|GetDamageAmount))
          (if (Variables|/Game/BPs/CharacterRelated/BP_MasterCharacter.BP_MasterCharacter_C|GetIsDead _as_bp_master_character)
            _
            (else
              (CallFunction|SpawnImpactFX _returnvalue "0, 0, 0" true _array_element)))
          (Game|SpawnActorfromClass "/Game/BPs/Items/Weapons/BP_Projectile.BP_Projectile_C" (Math|Transform|MakeTransform _returnvalue "0, 0, 0" "1.000000,1.000000,1.000000") "Undefined" 0 0)
          (Audio|PlaySoundatLocation "/Game/Sounds/SC_SlashHit.SC_SlashHit" _returnvalue "0, 0, 0" 1.0 1.0 0.0 0 0 0 0))
        (else
          (Audio|PlaySoundatLocation "/Game/Sounds/SC_Slash.SC_Slash" (Transformation|GetWorldLocation (Variables|Default|GetHitLocation)) "0, 0, 0" 1.0 1.0 0.0 0 0 0 0))))))

(event Custom|RotateTowardEnemy
  (params (ClosestEnemy :type BP%20Master%20Character%20Object%20Reference))
  (switch Utilities|FlowControl|Switch|SwitchonE_CameraType (Variables|/Game/BPs/CharacterRelated/BP_Player.BP_Player_C|GetCameraType (Variables|Default|GetAs%20BP%20Player))
    (:NewEnumerator0
      (if true
        (Utilities|IsValid ClosestEnemy
          (:Is%20Valid
            (if (not (Variables|/Game/BPs/CharacterRelated/BP_MasterCharacter.BP_MasterCharacter_C|GetIsDead ClosestEnemy))
              (bind _returnvalue (Utilities|Time|SetTimerbyEvent (delegate Custom|RotateTowardEnemyHandler) 0.01 true))
              (Variables|Default|SetRotateTimerHandle _returnvalue))))))))

(event Custom|RotateTowardEnemyHandler
  (CallFunction|RotatetoEnemy (stale Custom|RotateTowardEnemy ClosestEnemy)))

(event EventBeginPlay
  (|CallParentFunction))

(event EventUse
  (params (Instigator :type Actor%20Object%20Reference) (IsIA? :type Boolean))
  (Variables|Default|SetIs%20IA? IsIA?)
  (bind _asbp_player (Utilities|Casting|CastToBP_Player Instigator)
    (:then
      (bind _output_get (Variables|Default|SetAs%20BP%20Player _asbp_player))
      (Variables|Default|SetAs%20BP%20Master%20Character _output_get))
    (:CastFailed
      (bind _asbp_master_character (Utilities|Casting|CastToBP_MasterCharacter Instigator))
      (Variables|Default|SetAs%20BP%20Master%20Character _asbp_master_character)))
  (CallFunction|PlayAttack))

(event EventOnAimDown
  (params (Instigator :type BP%20Master%20Character%20Object%20Reference))
  (Variables|/Game/BPs/CharacterRelated/BP_MasterCharacter.BP_MasterCharacter_C|SetIsParrying Instigator true))

(event EventDestroyed
  (Utilities|WalkMode))

(event EventOnUnaim
  (params (Instigator :type BP%20Master%20Character%20Object%20Reference))
  (Variables|/Game/BPs/CharacterRelated/BP_MasterCharacter.BP_MasterCharacter_C|SetIsParrying Instigator false))

(fn ConstructionScript
  (|CallParentFunction))

(fn GetClosestEnemy
  (for _array_element (Collision|GetOverlappingActors (Variables|/Game/BPs/CharacterRelated/BP_MasterCharacter.BP_MasterCharacter_C|GetCloseRange (Variables|Default|GetAs%20BP%20Master%20Character)) "/Game/BPs/CharacterRelated/BP_MasterCharacter.BP_MasterCharacter_C" :!class /Script/Engine.PrimitiveComponent)
    (if (!= _array_element (Variables|Default|GetAs%20BP%20Master%20Character))
      (if (< (Math|Vector|Distance(Vector) (Transformation|GetActorLocation _array_element) (Transformation|GetActorLocation)) (LocalVariables|GetClosestDistance))
        (bind _asbp_master_character (Utilities|Casting|CastToBP_MasterCharacter _array_element))
        (LocalVariables|SetClosestEnemy _asbp_master_character))))
  (return (LocalVariables|GetClosestEnemy)))

(fn RotatetoEnemy
  (params (Enemy :type BP%20Master%20Character%20Object%20Reference))
  (bind _returnvalue (Transformation|GetActorLocation Enemy))
  (bind _as_bp_master_character (Variables|Default|GetAs%20BP%20Master%20Character))
  (bind _returnvalue_2 (Transformation|GetActorLocation _as_bp_master_character))
  (Transformation|SetActorRotation _as_bp_master_character (Math|Rotator|MakeRotator 0.0 0.0 (.yaw (Math|Rotator|FindLookatRotation _returnvalue_2 _returnvalue))))
  (if (Math|Boolean|ORBoolean (Variables|/Game/BPs/CharacterRelated/BP_MasterCharacter.BP_MasterCharacter_C|GetIsDead Enemy) (not (Variables|Default|GetIsAttacking)) (> (Math|Vector|Distance(Vector) _returnvalue_2 _returnvalue) 3e+02))
    (Utilities|Time|ClearandInvalidateTimerbyHandle (Variables|Default|GetRotateTimerHandle))))

(fn SpawnImpactFX
  (params (ImpactPoint :type Vector) (TraceEnd :type Vector) (Hit? :type Boolean) (HitActor :type Actor%20Object%20Reference))
  (bind _returnvalue (Math|Vector|SelectVector ImpactPoint TraceEnd Hit?))
  (bind _as_bp_master_character (Variables|Default|GetAs%20BP%20Master%20Character))
  (bind _rootcomponent (Variables|/Script/Engine.Actor|GetRootComponent _as_bp_master_character))
  (bind _returnvalue_2 (Transformation|GetWorldLocation _rootcomponent))
  (bind _returnvalue_3 (Math|Rotator|FindLookatRotation _returnvalue_2 _returnvalue))
  (bind _returnvalue_4 (- (.yaw _returnvalue_3) 1.8e+02))
  (bind _returnvalue_5 (Math|Rotator|MakeRotator (.roll _returnvalue_3) (.pitch _returnvalue_3) _returnvalue_4))
  (Utilities|Casting|CastToBP_MasterCharacter HitActor
    (:then
      (Game|SpawnActorfromClass "/Game/BPs/Items/Weapons/BP_ImpactPoint.BP_ImpactPoint_C" (Math|Transform|MakeTransform _returnvalue _returnvalue_5 "1.000000,1.000000,1.000000") "AlwaysSpawn" 0 true 0))
    (:CastFailed
      (Game|SpawnActorfromClass "/Game/BPs/Items/Weapons/BP_ImpactPoint.BP_ImpactPoint_C" (Math|Transform|MakeTransform _returnvalue _returnvalue_5 "1.000000,1.000000,1.000000") "AlwaysSpawn" 0 false 0))))