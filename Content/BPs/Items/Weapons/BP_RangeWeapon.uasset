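; Ranged weapon for player and AI characters, handling hitscan fire, ammo, timed reload and aim-down-sights alignment.
; Use fires only while a player owner aims, tracing from the camera or AI body, with spread for AI and eight-pellet shotguns.
; Player shots are re-traced by sphere from the weapon; hits deal damage, spawn impact FX and drop BP_Projectile on enemies.
; Reload plays montages and drives the HUD progress bar through a Tick gate.
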(event Custom|Reload
  (bind _as_bp_player (Variables|Default|GetAs%20BP%20Player))
  (bind _asplayerhud (Variables|/Game/BPs/CharacterRelated/BP_Player.BP_Player_C|GetAsPlayerHUD _as_bp_player))
  (bind _wbp_reload (Variables|/Game/BPs/WBPs/WBP_PlayerHUD.WBP_PlayerHUD_C|GetWBP_Reload _asplayerhud))
  (if (< (Variables|Default|GetBulletsInMag) (Variables|Default|GetMaxBulletsInMag))
    (Utilities|PlayReloadAnim
      (:Out
        (if (.bSuccess (Utilities|Casting|CastToBP_Player (Variables|Default|GetGunOwner)))
          (Widget|SetVisibility (Variables|/Game/BPs/WBPs/WBP_PlayerHUD.WBP_PlayerHUD_C|GetWBP_Reload (Variables|/Game/BPs/CharacterRelated/BP_Player.BP_Player_C|GetAsPlayerHUD (Variables|Default|GetAs%20BP%20Player))) "Visible")
          (else
            (Animation|Montage|PlayMontage (Variables|/Script/Engine.Character|GetMesh (.AsBP%20Master%20Enemy (Utilities|Casting|CastToBP_MasterEnemy (Variables|Default|GetGunOwner)))) "/Game/Characters/TPS/Animations/A_Reload_Rifle_Hip_Montage.A_Reload_Rifle_Hip_Montage"
              (:then
                _))))
        (Utilities|FlowControl|Sequence
          (:then_0
            (Utilities|FlowControl|Delay (Variables|Default|GetReloadTime))
            (Variables|Default|SetBulletsInMag (Variables|Default|GetMaxBulletsInMag))
            (Widget|SetVisibility _wbp_reload "Hidden")
            (Rendering|Material|SetScalarParameterValue (Variables|/Game/BPs/WBPs/WBP_Reload.WBP_Reload_C|GetPB_DynMat _wbp_reload) "Percent" 0.0 :!class /Script/Engine.MaterialInstanceDynamic)
            (Variables|/Game/BPs/WBPs/WBP_Reload.WBP_Reload_C|SetElpasedTime _wbp_reload 0.0)
            (Default|CallOnReload)
            (Utilities|FlowControl|Gate true) ; enters at Close
          )
          (:then_1
            (Utilities|FlowControl|Gate true) ; enters at Open
          ))))))

(event Custom|PlayFireAnimMontage
  (params (IsAI :type Boolean))
  (bind _gunowner (Variables|Default|GetGunOwner))
  (bind _asbp_player (Utilities|Casting|CastToBP_Player _gunowner))
  (if IsAI
    (Animation|Montage|PlayMontage (Variables|/Script/Engine.Character|GetMesh (Variables|Default|GetGunOwner)) (Variables|Default|GetTPS_IA_FireMontage) :!label _label)
    (else
      (switch Utilities|FlowControl|Switch|SwitchonE_CameraType (Variables|/Game/BPs/CharacterRelated/BP_Player.BP_Player_C|GetCameraType _asbp_player)
        (:NewEnumerator0
          (goto _label))
        (:NewEnumerator1
          (Animation|Montage|PlayMontage (Variables|/Game/BPs/CharacterRelated/BP_Player.BP_Player_C|GetFPS_Mesh _asbp_player) (Variables|Default|GetFPS_FireMontage) 0.5))))))

(event EventOnAimDown
  (params (Instigator :type BP%20Master%20Character%20Object%20Reference))
  (Default|WeaponAimDown (.AsBP%20Player (Utilities|Casting|CastToBP_Player (Game|Player|GetPlayerPawn 0)))))

(event EventOnUnaim
  (params (Instigator :type BP%20Master%20Character%20Object%20Reference))
  (Default|WeaponUnAim (.AsBP%20Player (Utilities|Casting|CastToBP_Player (Game|Player|GetPlayerPawn 0)))))

(event EventTick
  (params (DeltaSeconds :type Float%20%28single-precision%29))
  (if (.bSuccess (Utilities|Casting|CastToBP_Player (Variables|Default|GetGunOwner)))
    (Utilities|FlowControl|Gate true
      (:Exit
        (Default|SetPBValue (Variables|/Game/BPs/WBPs/WBP_PlayerHUD.WBP_PlayerHUD_C|GetWBP_Reload (Variables|/Game/BPs/CharacterRelated/BP_Player.BP_Player_C|GetAsPlayerHUD (Variables|Default|GetAs%20BP%20Player))) DeltaSeconds (Variables|Default|GetReloadTime))))))

(event EventUse
  (params (Instigator :type Actor%20Object%20Reference) (IsIA? :type Boolean))
  (bind _asbp_master_character (Utilities|Casting|CastToBP_MasterCharacter Instigator))
  (bind _output_get (Variables|Default|SetGunOwner _asbp_master_character))
  (bind _asbp_player (Utilities|Casting|CastToBP_Player _output_get)
    (:then
      (if (Variables|/Game/BPs/CharacterRelated/BP_Player.BP_Player_C|GetIsAiming _asbp_player)
        (Default|CallOnAmmoChange :!label _label)
        (if (Math|Boolean|ANDBoolean (> (Variables|Default|GetBulletsInMag) 0) (Variables|Default|GetCanShoot?) (Variables|/Game/BPs/CharacterRelated/BP_MasterCharacter.BP_MasterCharacter_C|GetCanShoot (Variables|Default|GetGunOwner)))
          (bind _hitresult (CallFunction|DoTrace (Variables|Default|GetGunOwner) IsIA?))
          (Utilities|FlowControl|Sequence
            (:then_0
              (Variables|Default|SetCanShoot? false)
              (Utilities|FlowControl|Delay (Variables|Default|GetFireRate))
              (Variables|Default|SetCanShoot? true))
            (:then_1
              (Components|Activation|Activate (Variables|Default|GetMuzzleFlash) true)
              (Variables|Default|SetBulletsInMag (- (Variables|Default|GetBulletsInMag) 1))
              (Default|CallOnAmmoChangeAI))
            (:then_2
              (for _array_element _hitresult
                (Utilities|FlowControl|Sequence
                  (:then_0
                    (bind _asbp_master_character_2 (Utilities|Casting|CastToBP_MasterCharacter (.HitActor (Collision|BreakHitResult _array_element))))
                    (Default|DealDamages (Variables|Default|GetGunOwner) _asbp_master_character_2 (Variables|Default|GetDamages)))
                  (:then_1
                    (CallFunction|SpawnImpactFX (.ImpactPoint (Collision|BreakHitResult _array_element)) (.TraceEnd (Collision|BreakHitResult _array_element)) false (.HitActor (Collision|BreakHitResult _array_element)))
                    (if (== (Utilities|GetClass (Variables|Default|GetGunOwner)) "/Game/BPs/CharacterRelated/BP_Player.BP_Player_C")
                      (Utilities|Casting|CastToBP_MasterEnemy (.HitActor (Collision|BreakHitResult _array_element)))
                      (Game|SpawnActorfromClass "/Game/BPs/Items/Weapons/BP_Projectile.BP_Projectile_C" (Math|Transform|MakeTransform (.ImpactPoint (Collision|BreakHitResult _array_element)) "0, 0, 0" "1.000000,1.000000,1.000000") "Undefined" 0 0))))))
            (:then_3
              (CallFunction|PlayFireAnimMontage IsIA?))))))
    (:CastFailed
      (goto _label))))

(event EventBeginPlay
  (bind _returnvalue (Game|Player|GetPlayerPawn 0))
  (bind (_asbp_player _bsuccess) (Utilities|Casting|CastToBP_Player _returnvalue))
  (bind _adsloc (Variables|/Game/BPs/CharacterRelated/BP_Player.BP_Player_C|GetADSLoc _asbp_player))
  (bind _relativelocation (Variables|/Script/Engine.SceneComponent|GetRelativeLocation _adsloc))
  (Variables|Default|SetAs%20BP%20Player _asbp_player)
  (if (and _bsuccess (Variables|/Game/BPs/CharacterRelated/BP_Player.BP_Player_C|GetIsAiming _asbp_player))
    (Default|WeaponAimDown _asbp_player)
    (else
      (Default|WeaponUnAim _asbp_player)))
  (Transformation|SetRelativeLocation _adsloc (Math|Vector|MakeVector (.x _relativelocation) (.y _relativelocation) (- (.z _relativelocation) (.z (Variables|/Script/Engine.SceneComponent|GetRelativeLocation (Variables|Default|GetAimLoc))))) false false)
  (Variables|Default|SetBulletsInMag (Variables|Default|GetMaxBulletsInMag)))

(event EventDestroyed
  (bind _returnvalue (Game|Player|GetPlayerPawn 0))
  (bind _as_bp_player (Variables|Default|GetAs%20BP%20Player))
  (bind _asbp_player (Utilities|Casting|CastToBP_Player _returnvalue))
  (bind _asplayerhud (Variables|/Game/BPs/CharacterRelated/BP_Player.BP_Player_C|GetAsPlayerHUD _as_bp_player))
  (bind _wbp_reload (Variables|/Game/BPs/WBPs/WBP_PlayerHUD.WBP_PlayerHUD_C|GetWBP_Reload _asplayerhud))
  (Transformation|SetRelativeLocation (Variables|/Game/BPs/CharacterRelated/BP_Player.BP_Player_C|GetADSLoc _asbp_player) (Variables|/Game/BPs/CharacterRelated/BP_Player.BP_Player_C|GetADS_BaseLoc _asbp_player) false false)
  (Widget|SetVisibility _wbp_reload "Hidden")
  (Variables|/Game/BPs/WBPs/WBP_Reload.WBP_Reload_C|SetElpasedTime _wbp_reload 0.0))

(fn ConstructionScript
  (|CallParentFunction))

(fn SpawnImpactFX
  (params (ImpactPoint :type Vector) (TraceEnd :type Vector) (Hit? :type Boolean) (HitActor :type Actor%20Object%20Reference))
  (bind _returnvalue (Math|Vector|SelectVector ImpactPoint TraceEnd Hit?))
  (bind _gunowner (Variables|Default|GetGunOwner))
  (bind _rootcomponent (Variables|/Script/Engine.Actor|GetRootComponent _gunowner))
  (bind _returnvalue_2 (Transformation|GetWorldLocation _rootcomponent))
  (bind _returnvalue_3 (Math|Rotator|FindLookatRotation _returnvalue_2 _returnvalue))
  (bind _returnvalue_4 (- (.yaw _returnvalue_3) 1.8e+02))
  (bind _returnvalue_5 (Math|Rotator|MakeRotator (.roll _returnvalue_3) (.pitch _returnvalue_3) _returnvalue_4))
  (Utilities|Casting|CastToBP_MasterCharacter HitActor
    (:then
      (Game|SpawnActorfromClass "/Game/BPs/Items/Weapons/BP_ImpactPoint.BP_ImpactPoint_C" (Math|Transform|MakeTransform _returnvalue _returnvalue_5 "1.000000,1.000000,1.000000") "AlwaysSpawn" 0 true 0))
    (:CastFailed
      (Game|SpawnActorfromClass "/Game/BPs/Items/Weapons/BP_ImpactPoint.BP_ImpactPoint_C" (Math|Transform|MakeTransform _returnvalue _returnvalue_5 "1.000000,1.000000,1.000000") "AlwaysSpawn" 0 false 0))))

(fn DoTrace
  (params (Character :type BP%20Master%20Character%20Object%20Reference) (IsAI :type Boolean))
  (bind _asbp_player (Utilities|Casting|CastToBP_Player Character))
  (bind _bulletrange (Variables|Default|GetBulletRange))
  (bind _returnvalue (Transformation|GetActorLocation Character))
  (bind _returnvalue_2 (Transformation|GetActorForwardVector Character))
  (bind _cameratype (Variables|/Game/BPs/CharacterRelated/BP_Player.BP_Player_C|GetCameraType _asbp_player))
  (bind _tps_camera (Variables|/Game/BPs/CharacterRelated/BP_Player.BP_Player_C|GetTPS_Camera _asbp_player))
  (bind _fps_camera (Variables|/Game/BPs/CharacterRelated/BP_Player.BP_Player_C|GetFPS_Camera _asbp_player))
  (bind _returnvalue_3 (Utilities|Select :Index _cameratype :NewEnumerator0 _tps_camera :NewEnumerator1 _fps_camera))
  (bind _returnvalue_4 (Transformation|GetWorldLocation _returnvalue_3))
  (bind _returnvalue_5 (Math|Vector|GetForwardVector _returnvalue_3))
  (bind _returnvalue_6 (select IsAI _returnvalue_2 _returnvalue_5))
  (bind _returnvalue_7 (select IsAI _returnvalue _returnvalue_4))
  (bind _returnvalue_8 (* _returnvalue_6 _bulletrange))
  (bind _returnvalue_9 (+ _returnvalue_7 _returnvalue_8))
  (if (Variables|Default|GetIsShotgun)
    (for _index (range 1 8)
      (bind (_outhit _returnvalue_10) (Collision|LineTraceByChannel _returnvalue_7 (select (or IsAI (Variables|Default|GetIsShotgun)) (CallFunction|SpreadTrace _returnvalue_9) _returnvalue_9) "TraceTypeQuery1" false (Utilities|Array|MakeArray (Variables|Default|GetGunOwner) self) "None"))
      (Utilities|Array|Add (LocalVariables|GetLinetraceResult) _outhit)
      (if (not (Variables|Default|GetIsShotgun))
        (if IsAI
          (return (LocalVariables|GetLinetraceResult))
          (else
            (for _array_element (LocalVariables|GetLinetraceResult)
              (bind _outhit_2 (Collision|SphereTraceByChannel (Transformation|GetActorLocation) (select _returnvalue_10 (.ImpactPoint (Collision|BreakHitResult _array_element)) (.TraceEnd (Collision|BreakHitResult _array_element))) 1e+01 "TraceTypeQuery1" false (Utilities|Array|MakeArray (Variables|Default|GetGunOwner) self) "None"))
              (Utilities|Array|Add (LocalVariables|GetSphereTraceResult) _outhit_2))
            (return (LocalVariables|GetSphereTraceResult))))))
    (if IsAI :!label _label
      (return (LocalVariables|GetLinetraceResult))
      (else
        (for _array_element_2 (LocalVariables|GetLinetraceResult)
          (bind _outhit_3 (Collision|SphereTraceByChannel (Transformation|GetActorLocation) (select _returnvalue_10 (.ImpactPoint (Collision|BreakHitResult _array_element_2)) (.TraceEnd (Collision|BreakHitResult _array_element_2))) 1e+01 "TraceTypeQuery1" false (Utilities|Array|MakeArray (Variables|Default|GetGunOwner) self) "None"))
          (Utilities|Array|Add (LocalVariables|GetSphereTraceResult) _outhit_3))
        (return (LocalVariables|GetSphereTraceResult))))
    (else
      (bind (_outhit_4 _returnvalue_11) (Collision|LineTraceByChannel _returnvalue_7 (select (or IsAI (Variables|Default|GetIsShotgun)) (CallFunction|SpreadTrace _returnvalue_9) _returnvalue_9) "TraceTypeQuery1" false (Utilities|Array|MakeArray (Variables|Default|GetGunOwner) self) "None"))
      (Utilities|Array|Add (LocalVariables|GetLinetraceResult) _outhit_4)
      (if (not (Variables|Default|GetIsShotgun))
        (goto _label)))))

(fn SpreadTrace
  (params (Vector :type Vector))
  (bind (_x _y _z) (Math|Vector|BreakVector Vector))
  (bind _spreadvalue (Variables|Default|GetSpreadValue))
  (bind _returnvalue (* _spreadvalue -1.0))
  (return (Math|Vector|MakeVector (+ _x (Math|Random|RandomFloatinRange _returnvalue _spreadvalue)) (+ _y (Math|Random|RandomFloatinRange _returnvalue _spreadvalue)) (+ _z (Math|Random|RandomFloatinRange _returnvalue _spreadvalue)))))