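; BP_Pistol is a pistol weapon Blueprint that supplies the firing animation for its owner.
; Its PlayFireAnimMontage event plays the single-shot standing fire montage on the owner's mesh when the wielder is AI.
; For players it casts the owner to BP_Player and uses CameraType to play the same montage on either the third-person mesh or the first-person FPSMesh.
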(event EventBeginPlay
  (|CallParentFunction) ; This node is disabled and will not be called.\nDrag off pins to build functionality.
)

(event Collision|EventActorBeginOverlap
  (params (OtherActor :type Actor%20Object%20Reference)))

(event EventTick
  (params (DeltaSeconds :type Float%20%28single-precision%29)))

(event EventPlayFireAnimMontage
  (params (IsAI :type Boolean))
  (bind _gunowner (Variables|Default|GetGunOwner))
  (bind _asbp_player (Utilities|Casting|CastToBP_Player _gunowner))
  (if IsAI
    (Animation|Montage|PlayMontage (Variables|/Script/Engine.Character|GetMesh (Variables|Default|GetGunOwner)) "/Game/Characters/TPS/Animations/Pistol/Fire/AM_W1_Stand_Fire_Single_Montage.AM_W1_Stand_Fire_Single_Montage")
    (else
      (switch Utilities|FlowControl|Switch|SwitchonE_CameraType (Variables|/Game/BPs/CharacterRelated/BP_Player.BP_Player_C|GetCameraType _asbp_player)
        (:NewEnumerator0
          (Animation|Montage|PlayMontage (Variables|/Script/Engine.Character|GetMesh _asbp_player) "/Game/Characters/TPS/Animations/Pistol/Fire/AM_W1_Stand_Fire_Single_Montage.AM_W1_Stand_Fire_Single_Montage"))
        (:NewEnumerator1
          (Animation|Montage|PlayMontage (Variables|/Game/BPs/CharacterRelated/BP_Player.BP_Player_C|GetFPS_Mesh _asbp_player) "/Game/Characters/TPS/Animations/Pistol/Fire/AM_W1_Stand_Fire_Single_Montage.AM_W1_Stand_Fire_Single_Montage"))))))

(fn ConstructionScript
  (|CallParentFunction))