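; BP_Food is a consumable item that heals the player who uses it.
; Use checks and locks the player's CanEat flag, waits ConsumptionTime, then sends HealMessage and unlocks eating.
; It then decrements the inventory wheel slot at the player's current index read after the delay, clearing it at zero or calling SpawnItem otherwise.
; Finally, it refreshes the HUD inventory slot and destroys itself.
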(event EventUse
  (params (Instigator :type Actor%20Object%20Reference) (IsIA? :type Boolean))
  (bind _asbp_player (Utilities|Casting|CastToBP_Player Instigator))
  (if (Variables|/Game/BPs/CharacterRelated/BP_Player.BP_Player_C|GetCanEat _asbp_player)
    (Variables|/Game/BPs/CharacterRelated/BP_Player.BP_Player_C|SetCanEat _asbp_player false)
    (Utilities|FlowControl|Delay (Variables|Default|GetConsumptionTime))
    (Class|BPICombat|Heal(Message) _asbp_player (Variables|Default|GetAmountToHeal))
    (Variables|/Game/BPs/CharacterRelated/BP_Player.BP_Player_C|SetCanEat _asbp_player true)
    (if (== (- (.quantity (Utilities|Array|Get(acopy) (Variables|/Game/BPs/CharacterRelated/BP_Player.BP_Player_C|GetPlayerInventoryWheel _asbp_player) (Variables|/Game/BPs/CharacterRelated/BP_Player.BP_Player_C|GetCurrentInventoryIndex _asbp_player))) 1) 0)
      (Utilities|Array|SetArrayElem (Variables|/Game/BPs/CharacterRelated/BP_Player.BP_Player_C|GetPlayerInventoryWheel _asbp_player) (Variables|/Game/BPs/CharacterRelated/BP_Player.BP_Player_C|GetCurrentInventoryIndex _asbp_player) (Utilities|Struct|MakeSTR_Inventory 0 0))
      (else
        (Utilities|Array|SetArrayElem (Variables|/Game/BPs/CharacterRelated/BP_Player.BP_Player_C|GetPlayerInventoryWheel _asbp_player) (Variables|/Game/BPs/CharacterRelated/BP_Player.BP_Player_C|GetCurrentInventoryIndex _asbp_player) (Utilities|Struct|MakeSTR_Inventory (.itemclass (Utilities|Array|Get(acopy) (Variables|/Game/BPs/CharacterRelated/BP_Player.BP_Player_C|GetPlayerInventoryWheel _asbp_player) (Variables|/Game/BPs/CharacterRelated/BP_Player.BP_Player_C|GetCurrentInventoryIndex _asbp_player))) (- (.quantity (Utilities|Array|Get(acopy) (Variables|/Game/BPs/CharacterRelated/BP_Player.BP_Player_C|GetPlayerInventoryWheel _asbp_player) (Variables|/Game/BPs/CharacterRelated/BP_Player.BP_Player_C|GetCurrentInventoryIndex _asbp_player))) 1)))
        (Default|SpawnItem _asbp_player true)))
    (Default|SetIteminSlot (Variables|/Game/BPs/WBPs/WBP_PlayerHUD.WBP_PlayerHUD_C|GetWBP_PlayerInventory (Variables|/Game/BPs/CharacterRelated/BP_Player.BP_Player_C|GetAsPlayerHUD _asbp_player)))
    (Actor|DestroyActor)))

(fn ConstructionScript
  (|CallParentFunction))