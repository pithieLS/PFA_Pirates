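; Telescope item that gives the player a zoomed scope view while aiming, in both third- and first-person camera modes.
; Aiming plays a per-mode timeline, which in TPS pushes the camera forward and hides the player mesh.
; When it finishes, it shows the scope widget, applies the scope FOV and hides the item and HUD.
; Unaiming, or destruction while the widget is valid, removes the overlay, reverses the timeline and restores FOV and visibility.
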(event EventOnAimDown
  (params (Instigator :type BP%20Master%20Character%20Object%20Reference))
  (bind _as_bp_player_0 (Variables|Default|GetAs%20BP%20Player_0))
  (if (Utilities|Enum|Equal(Enum) (Variables|/Game/BPs/CharacterRelated/BP_Player.BP_Player_C|GetCameraType (Variables|Default|GetAs%20BP%20Player_0)) "NewEnumerator1")
    (|CallParentFunction 0))
  (Variables|Default|SetIsScoping true)
  (switch Utilities|FlowControl|Switch|SwitchonE_CameraType (Variables|/Game/BPs/CharacterRelated/BP_Player.BP_Player_C|GetCameraType (Variables|Default|GetAs%20BP%20Player_0))
    (:NewEnumerator0
      (bind _lerpvalue (Timeline|ScopeTPSTimeline Play)
        (:Update
          (if (and (> _lerpvalue 0.9) (Variables|Default|GetIsScoping))
            (Rendering|SetVisibility (Variables|/Script/Engine.Character|GetMesh _as_bp_player_0) false false))
          (Transformation|SetRelativeLocation (Variables|/Game/BPs/CharacterRelated/BP_Player.BP_Player_C|GetTPS_Camera _as_bp_player_0) (Math|Vector|Lerp(Vector) (Variables|/Game/BPs/CharacterRelated/BP_Player.BP_Player_C|GetTPS_Cam_BaseLoc _as_bp_player_0) "390.000000,0.000000,50.000000" _lerpvalue) false false))
        (:Finished
          (if (== _lerpvalue 1.0)
            (bind _returnvalue (UserInterface|CreateWidget "/Game/BPs/WBPs/WBP_ScopeTelescope.WBP_ScopeTelescope_C"))
            (bind _output_get (Variables|Default|SetScopeWidget _returnvalue))
            (UserInterface|Viewport|AddtoViewport _output_get 0)
            (Camera|SetFieldOfView (Variables|/Game/BPs/CharacterRelated/BP_Player.BP_Player_C|GetTPS_Camera (Variables|Default|GetAs%20BP%20Player_0)) (Variables|Default|GetScopeFOV))
            (Widget|SetVisibility (Variables|/Game/BPs/CharacterRelated/BP_Player.BP_Player_C|GetAsPlayerHUD (Variables|Default|GetAs%20BP%20Player_0)) "Hidden")))))
    (:NewEnumerator1
      (bind _lerpvalue_2 (Timeline|ScopeFPSTimeline Play)
        (:Update
          (if (and (> _lerpvalue_2 0.9) (Variables|Default|GetIsScoping))
            (Rendering|SetVisibility (Variables|Default|GetItemMesh) true false)))
        (:Finished
          (if (== _lerpvalue_2 1.0)
            (bind _returnvalue_2 (UserInterface|CreateWidget "/Game/BPs/WBPs/WBP_ScopeTelescope.WBP_ScopeTelescope_C"))
            (bind _output_get_2 (Variables|Default|SetScopeWidget _returnvalue_2))
            (UserInterface|Viewport|AddtoViewport _output_get_2 0)
            (Camera|SetFieldOfView (Variables|/Game/BPs/CharacterRelated/BP_Player.BP_Player_C|GetFPS_Camera (Variables|Default|GetAs%20BP%20Player_0)) (Variables|Default|GetScopeFOV))
            (Rendering|SetVisibility (Variables|Default|GetItemMesh) false false)
            (Widget|SetVisibility (Variables|/Game/BPs/CharacterRelated/BP_Player.BP_Player_C|GetAsPlayerHUD (Variables|Default|GetAs%20BP%20Player_0)) "Hidden")))))))

(event EventOnUnaim
  (params (Instigator :type BP%20Master%20Character%20Object%20Reference))
  (bind _as_bp_player_0 (Variables|Default|GetAs%20BP%20Player_0))
  (if (Utilities|Enum|Equal(Enum) (Variables|/Game/BPs/CharacterRelated/BP_Player.BP_Player_C|GetCameraType (Variables|Default|GetAs%20BP%20Player_0)) "NewEnumerator1")
    (|CallParentFunction 0))
  (Variables|Default|SetIsScoping false)
  (Widget|RemovefromParent (Variables|Default|GetScopeWidget))
  (switch Utilities|FlowControl|Switch|SwitchonE_CameraType (Variables|/Game/BPs/CharacterRelated/BP_Player.BP_Player_C|GetCameraType (Variables|Default|GetAs%20BP%20Player_0))
    (:NewEnumerator0
      (Utilities|FlowControl|Sequence
        (:then_0
          (bind _lerpvalue (Timeline|ScopeTPSTimeline Reverse)
            (:Update
              (if (and (> _lerpvalue 0.9) (Variables|Default|GetIsScoping))
                (Rendering|SetVisibility (Variables|/Script/Engine.Character|GetMesh _as_bp_player_0) false false))
              (Transformation|SetRelativeLocation (Variables|/Game/BPs/CharacterRelated/BP_Player.BP_Player_C|GetTPS_Camera _as_bp_player_0) (Math|Vector|Lerp(Vector) (Variables|/Game/BPs/CharacterRelated/BP_Player.BP_Player_C|GetTPS_Cam_BaseLoc _as_bp_player_0) "390.000000,0.000000,50.000000" _lerpvalue) false false))
            (:Finished
              (if (== _lerpvalue 1.0)
                (bind _returnvalue (UserInterface|CreateWidget "/Game/BPs/WBPs/WBP_ScopeTelescope.WBP_ScopeTelescope_C"))
                (bind _output_get (Variables|Default|SetScopeWidget _returnvalue))
                (UserInterface|Viewport|AddtoViewport _output_get 0)
                (Camera|SetFieldOfView (Variables|/Game/BPs/CharacterRelated/BP_Player.BP_Player_C|GetTPS_Camera (Variables|Default|GetAs%20BP%20Player_0)) (Variables|Default|GetScopeFOV))
                (Widget|SetVisibility (Variables|/Game/BPs/CharacterRelated/BP_Player.BP_Player_C|GetAsPlayerHUD (Variables|Default|GetAs%20BP%20Player_0)) "Hidden")))))
        (:then_1
          (Rendering|SetVisibility (Variables|/Script/Engine.Character|GetMesh (Variables|Default|GetAs%20BP%20Player_0)) true false))
        (:then_2
          (Camera|SetFieldOfView (Variables|/Game/BPs/CharacterRelated/BP_Player.BP_Player_C|GetTPS_Camera (Variables|Default|GetAs%20BP%20Player_0)) (Variables|Default|GetBaseFOV) :!label _label)
          (Rendering|SetVisibility (Variables|Default|GetItemMesh) true false)
          (Widget|SetVisibility (Variables|/Game/BPs/CharacterRelated/BP_Player.BP_Player_C|GetAsPlayerHUD (Variables|Default|GetAs%20BP%20Player_0)) "Visible"))))
    (:NewEnumerator1
      (Utilities|FlowControl|Sequence
        (:then_0
          (bind _lerpvalue_2 (Timeline|ScopeFPSTimeline Reverse)
            (:Update
              (if (and (> _lerpvalue_2 0.9) (Variables|Default|GetIsScoping))
                (Rendering|SetVisibility (Variables|Default|GetItemMesh) true false)))
            (:Finished
              (if (== _lerpvalue_2 1.0)
                (bind _returnvalue_2 (UserInterface|CreateWidget "/Game/BPs/WBPs/WBP_ScopeTelescope.WBP_ScopeTelescope_C"))
                (bind _output_get_2 (Variables|Default|SetScopeWidget _returnvalue_2))
                (UserInterface|Viewport|AddtoViewport _output_get_2 0)
                (Camera|SetFieldOfView (Variables|/Game/BPs/CharacterRelated/BP_Player.BP_Player_C|GetFPS_Camera (Variables|Default|GetAs%20BP%20Player_0)) (Variables|Default|GetScopeFOV))
                (Rendering|SetVisibility (Variables|Default|GetItemMesh) false false)
                (Widget|SetVisibility (Variables|/Game/BPs/CharacterRelated/BP_Player.BP_Player_C|GetAsPlayerHUD (Variables|Default|GetAs%20BP%20Player_0)) "Hidden")))))
        (:then_1
          (goto _label))))))

(event EventBeginPlay
  (bind _output_get (Variables|Default|SetAs%20BP%20Player_0 (.AsBP%20Player (Utilities|Casting|CastToBP_Player (Game|Player|GetPlayerPawn 0)))))
  (Variables|Default|SetBaseFOV (Variables|/Script/Engine.CameraComponent|GetFieldOfView (Variables|/Game/BPs/CharacterRelated/BP_Player.BP_Player_C|GetTPS_Camera _output_get))))

(event EventDestroyed
  (bind _scopewidget (Variables|Default|GetScopeWidget))
  (Utilities|IsValid _scopewidget
    (:Is%20Valid
      (Widget|RemovefromParent _scopewidget)
      (CallFunction|OnUnaim))))

(event EventUse
  (params (Instigator :type Actor%20Object%20Reference) (IsIA? :type Boolean)))

(event EventReload)

(fn ConstructionScript
  (|CallParentFunction))