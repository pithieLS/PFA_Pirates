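; BP_Map is a held map item that shows a map screen while the player aims with it.
; On spawn it flags the player as holding both a map and a direction item, and clears both flags when destroyed.
; Aiming creates a WBP_Map widget and adds it to the viewport, and releasing aim removes that widget.
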(event EventBeginPlay
  (bind _returnvalue (Game|Player|GetPlayerPawn 0))
  (bind _asbp_player (Utilities|Casting|CastToBP_Player _returnvalue))
  (|CallParentFunction)
  (Variables|/Game/BPs/CharacterRelated/BP_Player.BP_Player_C|SetHasDirectionItemInHand _asbp_player true)
  (Variables|/Game/BPs/CharacterRelated/BP_Player.BP_Player_C|SetHasMapInHand _asbp_player true))

(event EventOnAimDown
  (params (Instigator :type BP%20Master%20Character%20Object%20Reference))
  (bind _returnvalue (UserInterface|CreateWidget "/Game/BPs/WBPs/WBP_Map.WBP_Map_C"))
  (UserInterface|Viewport|AddtoViewport _returnvalue 0))

(event EventOnUnaim
  (params (Instigator :type BP%20Master%20Character%20Object%20Reference))
  (Widget|RemovefromParent (stale EventOnAimDown _returnvalue)))

(event EventDestroyed
  (bind _returnvalue (Game|Player|GetPlayerPawn 0))
  (bind _asbp_player (Utilities|Casting|CastToBP_Player _returnvalue))
  (Variables|/Game/BPs/CharacterRelated/BP_Player.BP_Player_C|SetHasDirectionItemInHand _asbp_player false)
  (Variables|/Game/BPs/CharacterRelated/BP_Player.BP_Player_C|SetHasMapInHand _asbp_player false))

(fn ConstructionScript
  (|CallParentFunction))