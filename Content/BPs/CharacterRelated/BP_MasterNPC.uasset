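; BP_MasterNPC is a base NPC Blueprint that plays idle, interact and hit montages from its AnimationStruct.
; It starts the idle montage on BeginPlay.
; Interact plays its montage and adds InteractWidget to the viewport, while TakeDamages plays the hit montage.
; Both reactions return to idle through the montage's Notify Begin callback rather than on completion.
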(event Custom|PlayIdleMontage
  (Animation|Montage|PlayMontage (Variables|Character|GetMesh) (.Idle (Utilities|Struct|BreakSTR_Animation (Variables|Default|GetAnimationStruct)))))

(event EventInteract
  (params (Player :type BP%20Player%20Object%20Reference))
  (bind _notifyname (Animation|Montage|PlayMontage (Variables|Character|GetMesh) (.Interact (Utilities|Struct|BreakSTR_Animation (Variables|Default|GetAnimationStruct))))
    (:then
      (bind _returnvalue (UserInterface|CreateWidget (Variables|Default|GetInteractWidget)))
      (UserInterface|Viewport|AddtoViewport _returnvalue 0))
    (:OnNotifyBegin
      (switch name _notifyname
        (:NextAnim
          (CallFunction|PlayIdleMontage))))))

(event EventBeginPlay
  (CallFunction|PlayIdleMontage))

(event EventTakeDamages
  (params (DamageAmount :type Integer) (DamageAuthor :type Actor%20Object%20Reference))
  (bind _notifyname (Animation|Montage|PlayMontage (Variables|Character|GetMesh) (.Hit (Utilities|Struct|BreakSTR_Animation (Variables|Default|GetAnimationStruct))))
    (:OnNotifyBegin
      (switch name _notifyname
        (:NextAnim
          (CallFunction|PlayIdleMontage))))))

(fn ConstructionScript
  (|CallParentFunction))