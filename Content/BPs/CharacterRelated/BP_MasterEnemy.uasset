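; BP_MasterEnemy is the base enemy Blueprint, extending a parent class that provides damage and death handling.
; After the parent processes damage, a dead enemy casts the damage author to BP_Player and passes itself to that player's quest manager via QuestDone.
; On death, its mesh starts simulating physics and its capsule ignores the Pawn and Camera collision channels.
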(event EventBeginPlay
  (|CallParentFunction) ; This node is disabled and will not be called.\nDrag off pins to build functionality.
)

(event Collision|EventActorBeginOverlap
  (params (OtherActor :type Actor%20Object%20Reference))
  (|CallParentFunction OtherActor) ; This node is disabled and will not be called.\nDrag off pins to build functionality.
)

(event EventTick
  (params (DeltaSeconds :type Float%20%28single-precision%29))
  (|CallParentFunction DeltaSeconds) ; This node is disabled and will not be called.\nDrag off pins to build functionality.
)

(event EventOnDead
  (bind _capsulecomponent (Variables|Default|GetCapsuleComponent))
  (|CallParentFunction)
  (Physics|SetSimulatePhysics (Variables|Character|GetMesh) true)
  (Collision|SetCollisionResponsetoChannel _capsulecomponent "ECC_Pawn" "ECR_Ignore")
  (Collision|SetCollisionResponsetoChannel _capsulecomponent "ECC_Camera" "ECR_Ignore"))

(event EventTakeDamages
  (params (DamageAmount :type Integer) (DamageAuthor :type Actor%20Object%20Reference))
  (|CallParentFunction DamageAmount DamageAuthor)
  (if (Variables|Default|GetIsDead)
    (bind _asbp_player (Utilities|Casting|CastToBP_Player DamageAuthor))
    (Default|QuestDone (Variables|/Game/BPs/CharacterRelated/BP_Player.BP_Player_C|GetAC_QuestManager _asbp_player) self)))

(fn ConstructionScript
  (|CallParentFunction))