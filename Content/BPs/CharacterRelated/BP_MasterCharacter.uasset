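; BP_MasterCharacter is a base character Blueprint that defines health and combat events.
; TakeDamages lowers Health, floors it at zero and calls OnDead, which currently only prints a debug string.
; Heal sets Health to current plus healed amount minus HealthMax, rather than clamping to the maximum.
; PlayShootMontage and DealDamages are empty events, and the construction script is empty.
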(event Custom|PlayShootMontage
  (params (AnimToPlay :type Anim%20Montage%20Object%20Reference)))

(event Custom|OnDead
  (Development|PrintString "Hello"))

(event EventTakeDamages
  (params (DamageAmount :type Integer) (DamageAuthor :type Actor%20Object%20Reference))
  (bind _output_get (Variables|Default|SetHealth (Math|Integer|Max(Integer) (- (Variables|Default|GetHealth) DamageAmount))))
  (if (== _output_get 0)
    (CallFunction|OnDead)))

(event EventHeal
  (params (PVAmount :type Integer))
  (Variables|Default|SetHealth (- (+ (Variables|Default|GetHealth) PVAmount) (Variables|Default|GetHealthMax))))

(event EventDealDamages
  (params (ToWho :type Actor%20Object%20Reference) (DamageAmount :type Integer)))

(fn ConstructionScript)