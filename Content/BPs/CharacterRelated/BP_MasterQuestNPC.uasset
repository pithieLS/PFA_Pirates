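; Master quest NPC Blueprint that presents a quest to the player on interaction.
; Interact creates a WBP_Quest widget from the NPC's QuestName and QuestStruct and adds it to the viewport.
; It then immediately calls QuestDone on the player's ACQuestManager, passing itself.
; BeginPlay and the construction script only call their parent versions.
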(event EventBeginPlay
  (|CallParentFunction))

(event EventInteract
  (params (Player :type BP%20Player%20Object%20Reference))
  (bind _returnvalue (UserInterface|CreateWidget "/Game/BPs/WBPs/Quest/WBP_Quest.WBP_Quest_C" 0 (Variables|Default|GetQuestName) (Variables|Default|GetQuestStruct)))
  (UserInterface|Viewport|AddtoViewport _returnvalue 0)
  (Default|QuestDone (Variables|/Game/BPs/CharacterRelated/BP_Player.BP_Player_C|GetAC_QuestManager Player) self))

(fn ConstructionScript
  (|CallParentFunction))