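; Player-possessable sailboat pawn with physics-driven movement, an orbiting camera and a work-in-progress cannon aim preview.
; Throttle pushes the hull with mass-scaled force up to a max speed, while steering rotates the clamped rudder.
; Tick applies turning force at a thruster above a minimum speed, and possession switches sails to a fade material.
; Scope predicts right-side cannonball paths into a spline, but look-direction detection only prints yaw.
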(event Custom|TurnBoat
  (bind _leftrightthruster (Variables|Default|GetLeftRightThruster))
  ;[1 1 1] TurnBoat s'execute que quand la vélocité est supérieur à 200 sinon il tourne sur place car TurnBoat est dans le tick
  (if (> (Math|Vector|VectorLength (Transformation|GetVelocity)) 2e+02)
    (Class|PrimitiveComponent|AddForceatLocation (Variables|Default|GetHullMesh) (* (Math|Vector|GetRightVector _leftrightthruster) (* (Utilities|CalculateTurnRate) (stale Input|EnhancedActionEvents|EnhancedInputActionInpA_Boat_LeftRight ActionValue) (Physics|GetMass (Variables|Default|GetHullMesh)))) (Transformation|GetWorldLocation _leftrightthruster) "None")))

(event Input|EnhancedActionEvents|EnhancedInputActionInpA_Boat_LeftRight
  (params (ActionValue :type Float%20%28double-precision%29) (ElapsedSeconds :type Float%20%28double-precision%29) (TriggeredSeconds :type Float%20%28double-precision%29) (InputAction :type Input%20Action%20Object%20Reference :default "/Game/Input/Boat/Actions/InpA_Boat_LeftRight.InpA_Boat_LeftRight"))
  (:Triggered
    (Utilities|RotateSafran ActionValue)))

(event Input|EnhancedActionEvents|EnhancedInputActionInp_Boat_Scope
  (params (ActionValue :type Boolean) (ElapsedSeconds :type Float%20%28double-precision%29) (TriggeredSeconds :type Float%20%28double-precision%29) (InputAction :type Input%20Action%20Object%20Reference :default "/Game/Input/Boat/Actions/Inp_Boat_Scope.Inp_Boat_Scope"))
  (bind _startcannonballsright (Variables|Default|GetStartCannonBallsRight))
  (:Triggered
    (switch Utilities|FlowControl|Switch|SwitchonLookDirection (Variables|Default|GetLookDirection)
      (:NewEnumerator0
        (bind _outpathpositions (Class|GameplayStatics|BlueprintPredictProjectilePathbyTraceChannel (Transformation|GetWorldLocation _startcannonballsright) (* (Math|Vector|GetForwardVector _startcannonballsright) (Variables|Default|GetThrowSpeed)) true 25.0 "ECC_WorldDynamic" false (Utilities|Array|MakeArray self) "ForOneFrame" 2.0))
        (Spline|SetSplinePoints (Variables|Default|GetPreviewCannonShots) _outpathpositions "World" true)
        (AddComponent|AddSplineMeshComponent true)))))

(event Input|EnhancedActionEvents|EnhancedInputActionInpA_Boat_Look
  (params (ActionValue :type Vector%202D%20Structure) (ElapsedSeconds :type Float%20%28double-precision%29) (TriggeredSeconds :type Float%20%28double-precision%29) (InputAction :type Input%20Action%20Object%20Reference :default "/Game/Input/Boat/Actions/InpA_Boat_Look.InpA_Boat_Look"))
  ;[1 1 1] Pour tourner la caméra du bateau sur l'axe horizontal
  (:Triggered
    (Transformation|AddWorldRotation (Variables|Default|GetSpringArm) (Math|Rotator|MakeRotator 0.0 0.0 (* (.X (Math|Vector2D|BreakVector2D ActionValue)) (Utilities|Time|GetWorldDeltaSeconds) 1e+02)) false false)
    (bind _output_get (CallFunction|CheckWatchDirection))))

(event Input|EnhancedActionEvents|EnhancedInputActionInpA_Boat_Throttle
  (params (ActionValue :type Float%20%28double-precision%29) (ElapsedSeconds :type Float%20%28double-precision%29) (TriggeredSeconds :type Float%20%28double-precision%29) (InputAction :type Input%20Action%20Object%20Reference :default "/Game/Input/Boat/Actions/InpA_Boat_Throttle.InpA_Boat_Throttle"))
  (bind _hullmesh (Variables|Default|GetHullMesh))
  (:Triggered
    (if (<= (Math|Vector|VectorLength (Transformation|GetVelocity)) (Variables|Default|GetMaxSpeed))
      (Physics|AddForce _hullmesh (* (Math|Vector|GetRightVector _hullmesh) (* (Physics|GetMass _hullmesh) (Variables|Default|GetAccelerationValue) ActionValue)) "None" false))))

(event EventPossessed
  (params (NewController :type Controller%20Object%20Reference))
  (Utilities|Casting|CastToPlayerController NewController)
  (Rendering|Material|SetMaterial (Variables|Default|GetSM_GrandeVoile) 0 "/Game/Materials/Boat/M_Sail_Fade.M_Sail_Fade"))

(event EventBeginPlay
  (bind _asplayer_controller (Utilities|Casting|CastToPlayerController (Pawn|GetController)))
  (Utilities|IsValid (PlayerController|LocalPlayerSubsystems|GetEnhancedInputLocalPlayerSubsystem _asplayer_controller)
    (:Is%20Valid
      (Input|AddMappingContext (PlayerController|LocalPlayerSubsystems|GetEnhancedInputLocalPlayerSubsystem _asplayer_controller) "/Game/Input/Boat/MC_Boat.MC_Boat" 0 "(bIgnoreAllPressedKeysUntilRelease=True,bForceImmediately=False)"))))

(event EventTick
  (params (DeltaSeconds :type Float%20%28single-precision%29))
  (Utilities|FlowControl|Sequence
    (:then_0
      (CallFunction|TurnBoat))))

(event EventUnpossessed
  (params (OldController :type Controller%20Object%20Reference))
  (Utilities|Casting|CastToPlayerController OldController)
  (Rendering|Material|SetMaterial (Variables|Default|GetSM_GrandeVoile) 0 "/Game/Materials/Boat/M_Sail.M_Sail"))

(fn ConstructionScript)

(fn CheckWatchDirection
  (Development|PrintString (Utilities|String|ToString(Float) (.yaw (Math|Interpolation|RInterpTo (Variables|/Script/Engine.SceneComponent|GetRelativeRotation (Variables|Default|GetSpringArm)) "0, 0, 0" (Utilities|Time|GetWorldDeltaSeconds) 3.0)))))