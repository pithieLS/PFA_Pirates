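; AI-controlled boat pawn that, on BeginPlay, uses an AIMoveTo through IA_BoatController to head for the player-style BP_Boat, printing success or failure.
; It carries physics thrust and turn forces, broadside cannon firing and spline-mesh trajectory previews built from projectile path prediction.
; These sailing, turning and aiming chains are disconnected from any live event, and Tick is empty, so only the move-to runs.
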(event Custom|TurnBoat
  (bind _leftrightthruster (Variables|Default|GetLeftRightThruster))
  ;[1 1 1] TurnBoat s'execute que quand la vélocité est supérieur à 200 sinon il tourne sur place car TurnBoat est dans le tick
  (if (> (Math|Vector|VectorLength (Transformation|GetVelocity)) 2e+02)
    (Class|PrimitiveComponent|AddForceatLocation (Variables|Default|GetHullMesh) (* (Math|Vector|GetRightVector _leftrightthruster) (* (Utilities|CalculateTurnRate) 0.0 (Physics|GetMass (Variables|Default|GetHullMesh)))) (Transformation|GetWorldLocation _leftrightthruster) "None")))

(event Input|EnhancedActionEvents|EnhancedInputActionInp_Boat_Scope
  (params (ActionValue :type Boolean) (ElapsedSeconds :type Float%20%28double-precision%29) (TriggeredSeconds :type Float%20%28double-precision%29) (InputAction :type Input%20Action%20Object%20Reference :default "/Game/Input/Boat/Actions/Inp_Boat_Scope.Inp_Boat_Scope")))

(event Input|EnhancedActionEvents|EnhancedInputActionInpA_Boat_WheelUp
  (params (ActionValue :type Float%20%28double-precision%29) (ElapsedSeconds :type Float%20%28double-precision%29) (TriggeredSeconds :type Float%20%28double-precision%29) (InputAction :type Input%20Action%20Object%20Reference :default "/Game/Input/Boat/Actions/InpA_Boat_WheelUp.InpA_Boat_WheelUp")))

(event Input|EnhancedActionEvents|EnhancedInputActionInpA_Boat_Shoot
  (params (ActionValue :type Boolean) (ElapsedSeconds :type Float%20%28double-precision%29) (TriggeredSeconds :type Float%20%28double-precision%29) (InputAction :type Input%20Action%20Object%20Reference :default "/Game/Input/Boat/Actions/InpA_Boat_Shoot.InpA_Boat_Shoot")))

(event EventBeginPlay
  (bind _returnvalue (Actor|GetActorOfClass "/Game/BPs/Boat/BP_Boat.BP_Boat_C"))
  (bind _asia_boat_controller (Utilities|Casting|CastToIA_BoatController (AI|GetAIController self)))
  (AI|AIMoveTo _asia_boat_controller (Transformation|GetActorLocation _returnvalue) _returnvalue -1.0 "Default" "Default" true true
    (:OnRequestFailed
      (Development|PrintString "Failed"))
    (:OnMoveFinished
      (Development|PrintString "Finished"))))

(event EventTick
  (params (DeltaSeconds :type Float%20%28single-precision%29)))

(fn ConstructionScript)

(fn RightCannonsShoot
  (bind _cannonsarray (Variables|Default|GetCannonsArray))
  (Utilities|Array|Clear (Variables|Default|GetCannonsArray))
  (Utilities|Array|Add _cannonsarray (Variables|/Script/Engine.ChildActorComponent|GetChildActor (Variables|Default|GetRightCannon)))
  (Utilities|Array|Add _cannonsarray (Variables|/Script/Engine.ChildActorComponent|GetChildActor (Variables|Default|GetRightCannon1)))
  (Utilities|Array|Add _cannonsarray (Variables|/Script/Engine.ChildActorComponent|GetChildActor (Variables|Default|GetRightCannon2)))
  (Utilities|Array|Add _cannonsarray (Variables|/Script/Engine.ChildActorComponent|GetChildActor (Variables|Default|GetRightCannon3)))
  (Utilities|Array|Add _cannonsarray (Variables|/Script/Engine.ChildActorComponent|GetChildActor (Variables|Default|GetRightCannon4)))
  (for _array_element (Variables|Default|GetCannonsArray)
    (bind _ascannons (Utilities|Casting|CastToCannons _array_element))
    (Default|Shoot _ascannons (Variables|Throw|GetZVector) (Variables|Throw|GetThrowSpeed)))
  (return))

(fn LeftCannonsShoot
  (bind _cannonsarray (Variables|Default|GetCannonsArray))
  (Utilities|Array|Clear (Variables|Default|GetCannonsArray))
  (Utilities|Array|Add _cannonsarray (Variables|/Script/Engine.ChildActorComponent|GetChildActor (Variables|Default|GetLeftCannon1)))
  (Utilities|Array|Add _cannonsarray (Variables|/Script/Engine.ChildActorComponent|GetChildActor (Variables|Default|GetLeftCannon2)))
  (Utilities|Array|Add _cannonsarray (Variables|/Script/Engine.ChildActorComponent|GetChildActor (Variables|Default|GetLeftCannon3)))
  (Utilities|Array|Add _cannonsarray (Variables|/Script/Engine.ChildActorComponent|GetChildActor (Variables|Default|GetLeftCannon4)))
  (Utilities|Array|Add _cannonsarray (Variables|/Script/Engine.ChildActorComponent|GetChildActor (Variables|Default|GetLeftCannon)))
  (for _array_element (Variables|Default|GetCannonsArray)
    (bind _ascannons (Utilities|Casting|CastToCannons _array_element))
    (Default|Shoot _ascannons (Variables|Throw|GetZVector) (Variables|Throw|GetThrowSpeed)))
  (return))

(fn Accelerate
  (bind _hullmesh (Variables|Default|GetHullMesh))
  (if (<= (Math|Vector|VectorLength (Transformation|GetVelocity)) (Variables|Default|GetMaxSpeed))
    (Physics|AddForce _hullmesh (* (Math|Vector|GetRightVector _hullmesh) (* (Physics|GetMass _hullmesh) (Variables|Throw|GetAccelerationValue) (Variables|Default|GetMaxAccel))) "None" false)
    (if (> (+ (Variables|Default|GetMaxAccel) 0.5) 1e+01)
      (Variables|Default|SetMaxAccel 1e+01)
      (else
        (Variables|Default|SetMaxAccel (+ (Variables|Default|GetMaxAccel) 0.5))))))

(fn Decelerate
  (bind _hullmesh (Variables|Default|GetHullMesh))
  (if (not (<= (Math|Vector|VectorLength (Transformation|GetVelocity)) 0.0))
    (Physics|AddForce _hullmesh (/ (Math|Vector|GetRightVector _hullmesh) (Utilities|Operators|Divide (Physics|GetMass _hullmesh) (Variables|Throw|GetAccelerationValue) (Variables|Default|GetMaxAccel))) "None" false)
    (if (< (- (Variables|Default|GetMaxAccel) 0.5) 0.0)
      (Variables|Default|SetMaxAccel -1.0)
      (else
        (Variables|Default|SetMaxAccel (- (Variables|Default|GetMaxAccel) 0.5))))))