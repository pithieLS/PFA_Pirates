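; Quest manager component that tracks a single active quest step and signals when it is completed.
; InitQuest stores the incoming step struct and prints its fields for debugging.
; QuestDone switches on quest type, matches the target against the stored actor (kills also require a BP_MasterEnemy), then clears the quest and shows a TaskCompleted widget.
; Only Talk and Kill have completion logic, although the struct also carries place and item objectives.
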(fn InitQuest
  (params (Quest :type STR%20Etape%20Structure))
  (bind (_actortotalk _actortokill _placetoreach _itemtopickup _questtype _stepdone_ _questdescription) (Utilities|Struct|BreakSTR_Etape Quest))
  (bind _output_get (Variables|Default|SetQuest (Utilities|Struct|MakeSTR_Etape _actortotalk _actortokill _placetoreach _itemtopickup _questtype _stepdone_ _questdescription)))
  (Development|PrintString (Utilities|String|Append "Actor To Talk : " (Utilities|GetDisplayName (.ActorToTalk (Utilities|Struct|BreakSTR_Etape _output_get))) " 
Actor To Kill : " (Utilities|GetDisplayName (.ActorToKill (Utilities|Struct|BreakSTR_Etape _output_get))) " 
Place To Reach :" (Utilities|String|ToString(Transform) (.PlaceToReach (Utilities|Struct|BreakSTR_Etape _output_get))) " 
Item To pick Up : " (Utilities|GetDisplayName (.ItemToPickUp (Utilities|Struct|BreakSTR_Etape _output_get))) " 
StepDone?" (Utilities|String|ToString(Boolean) (.StepDone? (Utilities|Struct|BreakSTR_Etape _output_get))) " 
Quest Description : " (Utilities|String|ToString(Text) (.QuestDescription (Utilities|Struct|BreakSTR_Etape _output_get))))))

(fn QuestDone
  (params (Target :type Actor%20Object%20Reference))
  (switch Utilities|FlowControl|Switch|SwitchonEnum_QuestType (.QuestType (Utilities|Struct|BreakSTR_Etape (Variables|Default|GetQuest)))
    (:NewEnumerator0
      (if (== (.ActorToTalk (Utilities|Struct|BreakSTR_Etape (Variables|Default|GetQuest))) Target)
        (Variables|Default|SetQuest "")
        (bind _returnvalue (UserInterface|CreateWidget "/Game/BPs/WBPs/Quest/TaskCompleted.TaskCompleted_C"))
        (UserInterface|Viewport|AddtoViewport _returnvalue 0)))
    (:NewEnumerator1
      (if (== (.ActorToKill (Utilities|Struct|BreakSTR_Etape (Variables|Default|GetQuest))) Target)
        (Utilities|Casting|CastToBP_MasterEnemy Target)
        (Variables|Default|SetQuest "")
        (bind _returnvalue_2 (UserInterface|CreateWidget "/Game/BPs/WBPs/Quest/TaskCompleted.TaskCompleted_C"))
        (UserInterface|Viewport|AddtoViewport _returnvalue_2 0)))))